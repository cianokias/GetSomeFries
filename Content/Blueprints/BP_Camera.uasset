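; BP_Camera is an actor that follows the first player character at a fixed offset.
; On BeginPlay it stores the difference between its own location and the character's location.
; Every Tick it moves to the character's location plus that offset, without sweep, interpolation or any change to its rotation.
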(event `self.ReceiveBeginPlay`
  (set `self.difference` (- (`self.K2_GetActorLocation`) (`self.K2_GetActorLocation` (`GameplayStatics.GetPlayerCharacter` 0)))))

(event `self.ReceiveTick`
  (params (DeltaSeconds :type "Float (single-precision)"))
  (`self.K2_SetActorLocation` (+ (`self.K2_GetActorLocation` (`GameplayStatics.GetPlayerCharacter` 0)) (`self.difference`))))

(fn `UserConstructionScript`)