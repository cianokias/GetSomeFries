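; Tutorial trigger box that ends the tutorial and loads the main level once the player seagull carries the fries.
; When a seagull overlaps the box, it polls the player every 0.1 seconds until the held item is "fries_t", even if the bird has left the box.
; It then disables control, calls FadeOut on the blackscreen UI, drops the item and opens the level after short delays.
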(event `self.Box.OnComponentBeginOverlap`
  (params (OverlappedComponent :type "PrimitiveComponent Object Reference") (OtherActor :type "Actor Object Reference") (OtherComp :type "PrimitiveComponent Object Reference") (OtherBodyIndex :type Integer) (bFromSweep :type Boolean) (SweepResult :type "HitResult Structure (by ref)"))
  (cast `/Game/Blueprints/BP_Seagull` OtherActor)
  (bind _asbp_seagull (cast `/Game/Blueprints/BP_Seagull` (`GameplayStatics.GetPlayerCharacter` 0) :!label _label))
  (if (`KismetStringLibrary.EqualEqual_StrStr` (`/Game/Blueprints/BP_Seagull.PickedItemId` _asbp_seagull) "fries_t")
    (set `/Game/Blueprints/BP_Seagull.canControl` false _asbp_seagull)
    (`KismetSystemLibrary.Delay` 0.5)
    (`/Game/Blueprints/UI/UI_BlackScreen.Fade Out` (`/Game/Blueprints/BP_Seagull.UI_Blackscreen_var` _asbp_seagull))
    (`KismetSystemLibrary.Delay` 1.0)
    (`/Game/Blueprints/BP_Seagull.Drop Item` _asbp_seagull)
    (`GameplayStatics.OpenLevelBySoftObjectPtr` "/Game/Maps/MainLevel.MainLevel")
    (else
      (`KismetSystemLibrary.Delay` 0.1)
      (goto _label))))

(event `self.Box.OnComponentEndOverlap`
  (params (OverlappedComponent :type "PrimitiveComponent Object Reference") (OtherActor :type "Actor Object Reference") (OtherComp :type "PrimitiveComponent Object Reference") (OtherBodyIndex :type Integer)))

(fn `UserConstructionScript`)