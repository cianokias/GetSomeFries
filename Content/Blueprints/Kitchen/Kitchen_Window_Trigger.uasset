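; Kitchen window exit trigger that sends the player seagull to the main level when it overlaps one of three boxes.
; Each overlap disables the seagull's control, fast-fades the screen out and waits briefly before the level loads.
; Box and Box1 share one main-level spawn point and Box2 uses another, stored in the master game instance before loading.
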(event `self.Box1.OnComponentBeginOverlap`
  (params (OverlappedComponent :type "PrimitiveComponent Object Reference") (OtherActor :type "Actor Object Reference") (OtherComp :type "PrimitiveComponent Object Reference") (OtherBodyIndex :type Integer) (bFromSweep :type Boolean) (SweepResult :type "HitResult Structure (by ref)"))
  (bind _asbp_seagull (cast `/Game/Blueprints/BP_Seagull` OtherActor))
  (set `/Game/Blueprints/BP_Seagull.canControl` false _asbp_seagull)
  (`/Game/Blueprints/UI_BlackScreen.FastFadeOut` (`/Game/Blueprints/BP_Seagull.UI_Blackscreen_var` _asbp_seagull))
  (`KismetSystemLibrary.Delay` 0.5)
  (bind _asgame_instance_master (cast `/Game/Blueprints/GameInstance_Master` (`GameplayStatics.GetGameInstance`) :!label _label))
  (set `/Game/Blueprints/GameInstance_Master.MainLevel_SpawnPoint` 1 _asgame_instance_master)
  (`GameplayStatics.OpenLevelBySoftObjectPtr` "/Game/Maps/MainLevel.MainLevel" :!label _label_2))

(event `self.Box.OnComponentBeginOverlap`
  (params (OverlappedComponent :type "PrimitiveComponent Object Reference") (OtherActor :type "Actor Object Reference") (OtherComp :type "PrimitiveComponent Object Reference") (OtherBodyIndex :type Integer) (bFromSweep :type Boolean) (SweepResult :type "HitResult Structure (by ref)"))
  (bind _asbp_seagull (cast `/Game/Blueprints/BP_Seagull` OtherActor))
  (set `/Game/Blueprints/BP_Seagull.canControl` false _asbp_seagull)
  (`/Game/Blueprints/UI_BlackScreen.FastFadeOut` (`/Game/Blueprints/BP_Seagull.UI_Blackscreen_var` _asbp_seagull))
  (`KismetSystemLibrary.Delay` 0.5)
  (goto _label))

(event `self.Box2.OnComponentBeginOverlap`
  (params (OverlappedComponent :type "PrimitiveComponent Object Reference") (OtherActor :type "Actor Object Reference") (OtherComp :type "PrimitiveComponent Object Reference") (OtherBodyIndex :type Integer) (bFromSweep :type Boolean) (SweepResult :type "HitResult Structure (by ref)"))
  (bind _asbp_seagull (cast `/Game/Blueprints/BP_Seagull` OtherActor))
  (set `/Game/Blueprints/BP_Seagull.canControl` false _asbp_seagull)
  (`/Game/Blueprints/UI_BlackScreen.FastFadeOut` (`/Game/Blueprints/BP_Seagull.UI_Blackscreen_var` _asbp_seagull))
  (`KismetSystemLibrary.Delay` 0.5)
  (bind _asgame_instance_master (cast `/Game/Blueprints/GameInstance_Master` (`GameplayStatics.GetGameInstance`)))
  (set `/Game/Blueprints/GameInstance_Master.MainLevel_SpawnPoint` 2 _asgame_instance_master)
  (goto _label_2))

(fn `UserConstructionScript`)