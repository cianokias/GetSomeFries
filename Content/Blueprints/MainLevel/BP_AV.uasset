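; BP_AV is a main-level actor that acts as an alarm reacting to BP_item actors entering its detection mesh.
; An overlap on StaticMesh1 swaps the material on StaticMesh and plays an attenuated alarm sound at the actor's location.
; The material changes again after a short delay, and an InDanger flag blocks retriggering until then.
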(event `self.StaticMesh1.OnComponentBeginOverlap`
  (params (OverlappedComponent :type "PrimitiveComponent Object Reference") (OtherActor :type "Actor Object Reference") (OtherComp :type "PrimitiveComponent Object Reference") (OtherBodyIndex :type Integer) (bFromSweep :type Boolean) (SweepResult :type "HitResult Structure (by ref)"))
  (cast `/Game/Blueprints/PickupSys/BP_item` OtherActor)
  (if (not (`self.inDanger`))
    (set `self.inDanger` true)
    (`PrimitiveComponent.SetMaterial` (`self.StaticMesh`) 0 "/Game/3DModels/Kitchen/Materials/B_R.B_R")
    (`GameplayStatics.PlaySoundAtLocation` "/Game/Music/alarm.alarm" (`self.K2_GetActorLocation`) (struct) 0.7 1.0 0.0 "/Game/Music/SA_Distence_radio.SA_Distence_radio" null null null)
    (`KismetSystemLibrary.Delay` 2.0)
    (`PrimitiveComponent.SetMaterial` (`self.StaticMesh`) 0 "/Game/3DModels/MainLevel/Beach_Plankroad/Rdiao/Material/R_PI.R_PI")
    (set `self.inDanger` false)))

(fn `UserConstructionScript`)