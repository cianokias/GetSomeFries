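; BP_Radio is a radio in the main level that the seagull player can switch between three songs and a soundless setting.
; A box overlap enables input and highlights the action tip, and the Action press advances the GameInstance track index, swapping screen material and sound.
; A looping timer tracks playback position, saved on EndPlay and resumed on BeginPlay.
; A sphere overlap starts an endless per-tick player-vector update, unused in this graph.
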(event `self.Sphere.OnComponentBeginOverlap`
  (params (OverlappedComponent :type "PrimitiveComponent Object Reference") (OtherActor :type "Actor Object Reference") (OtherComp :type "PrimitiveComponent Object Reference") (OtherBodyIndex :type Integer) (bFromSweep :type Boolean) (SweepResult :type "HitResult Structure (by ref)"))
  (cast `/Game/Blueprints/BP_Seagull` OtherActor)
  (set `self.inRange` true)
  (bind _output_get (set `self.PlayerLoc` (`self.K2_GetActorLocation` (`GameplayStatics.GetPlayerCharacter` 0)) :!label _label))
  (set `self.Playervector` (- _output_get (`self.K2_GetActorLocation`)))
  (`KismetSystemLibrary.DelayUntilNextTick`)
  (goto _label))

(event `self.Sphere.OnComponentEndOverlap`
  (params (OverlappedComponent :type "PrimitiveComponent Object Reference") (OtherActor :type "Actor Object Reference") (OtherComp :type "PrimitiveComponent Object Reference") (OtherBodyIndex :type Integer))
  (cast `/Game/Blueprints/BP_Seagull` OtherActor)
  (set `self.inRange` false))

(event `self.Box.OnComponentBeginOverlap`
  (params (OverlappedComponent :type "PrimitiveComponent Object Reference") (OtherActor :type "Actor Object Reference") (OtherComp :type "PrimitiveComponent Object Reference") (OtherBodyIndex :type Integer) (bFromSweep :type Boolean) (SweepResult :type "HitResult Structure (by ref)"))
  (bind _asbp_seagull (cast `/Game/Blueprints/BP_Seagull` OtherActor))
  (`self.EnableInput` (`GameplayStatics.GetPlayerController` 0))
  (`PrimitiveComponent.SetMaterial` (`/Game/Blueprints/BP_Seagull.actionTip_part` _asbp_seagull) 0 "/Game/Materials/MI_Solid_Yellow.MI_Solid_Yellow")
  (`PrimitiveComponent.SetMaterial` (`/Game/Blueprints/BP_Seagull.actionTip` _asbp_seagull) 0 "/Game/Materials/MI_Solid_Yellow.MI_Solid_Yellow"))

(event `self.Box.OnComponentEndOverlap`
  (params (OverlappedComponent :type "PrimitiveComponent Object Reference") (OtherActor :type "Actor Object Reference") (OtherComp :type "PrimitiveComponent Object Reference") (OtherBodyIndex :type Integer))
  (bind _asbp_seagull (cast `/Game/Blueprints/BP_Seagull` OtherActor))
  (`self.DisableInput` (`GameplayStatics.GetPlayerController` 0))
  (`PrimitiveComponent.SetMaterial` (`/Game/Blueprints/BP_Seagull.actionTip` _asbp_seagull) 0 "/Game/Materials/MI_Transparent_Inst.MI_Transparent_Inst")
  (`PrimitiveComponent.SetMaterial` (`/Game/Blueprints/BP_Seagull.actionTip_part` _asbp_seagull) 0 "/Game/Materials/MI_Transparent_Inst.MI_Transparent_Inst"))

(event `InputAction|Action`
  (params (Key :type "Key Structure"))
  (bind _audio (`self.Audio`))
  (:`Pressed`
    (bind _asgame_instance_master (cast `/Game/Blueprints/GameInstance_Master` (`GameplayStatics.GetGameInstance`)))
    (bind _output_get (set `/Game/Blueprints/GameInstance_Master.CurrentBGM` (+ (`/Game/Blueprints/GameInstance_Master.CurrentBGM` _asgame_instance_master) 1) _asgame_instance_master))
    (if (> _output_get 3)
      (set `/Game/Blueprints/GameInstance_Master.CurrentBGM` 0 _asgame_instance_master))
    (set `self.newsong` true)
    (set `self.timer` 0.0)
    (bind _asgame_instance_master_2 (cast `/Game/Blueprints/GameInstance_Master` (`GameplayStatics.GetGameInstance`) :!label _label_2))
    (bind _currentbgm (`/Game/Blueprints/GameInstance_Master.CurrentBGM` _asgame_instance_master_2))
    (`PrimitiveComponent.SetMaterial` (`self.SkeletalMesh`) 1 (select `int` _currentbgm :`0` "/Game/3DModels/MainLevel/Beach_Plankroad/Rdiao/Material/R_Screen_0.R_Screen_0" :`1` "/Game/3DModels/MainLevel/Beach_Plankroad/Rdiao/Material/R_Screen_1.R_Screen_1" :`2` "/Game/3DModels/MainLevel/Beach_Plankroad/Rdiao/Material/R_Screen_2.R_Screen_2" :`3` "/Game/3DModels/MainLevel/Beach_Plankroad/Rdiao/Material/R_Screen_3.R_Screen_3" :`4` null :!type "MaterialInterface Object Reference"))
    (`AudioComponent.SetSound` _audio (select `int` _currentbgm :`0` null :`1` "/Game/Music/upbeat1_Cue.upbeat1_Cue" :`2` "/Game/Music/upbeat2_Cue.upbeat2_Cue" :`3` "/Game/Music/bgm3_Cue.bgm3_Cue" :`4` null :!type "SoundBase Object Reference"))
    (`AudioComponent.Play` _audio (select `bool` (`self.newsong`) :`false` (`self.timer`) :!type "Float (single-precision)"))
    (`KismetSystemLibrary.K2_SetTimerDelegate` (delegate `SetTimer`) 0.05 true)))

(event `self.ReceiveBeginPlay`
  (bind _asgame_instance_master (cast `/Game/Blueprints/GameInstance_Master` (`GameplayStatics.GetGameInstance`)))
  (set `self.timer` (`/Game/Blueprints/GameInstance_Master.CurrentBGMTimer` _asgame_instance_master))
  (set `self.newsong` false)
  (goto _label_2))

(event `self.ReceiveEndPlay`
  (params (EndPlayReason :type "EEndPlayReason Enum" :default "Destroyed"))
  (bind _asgame_instance_master (cast `/Game/Blueprints/GameInstance_Master` (`GameplayStatics.GetGameInstance`)))
  (set `/Game/Blueprints/GameInstance_Master.CurrentBGMTimer` (`self.timer`) _asgame_instance_master))

(event `SetTimer`
  (set `self.timer` (+ (`self.timer`) 0.05)))

(fn `UserConstructionScript`)