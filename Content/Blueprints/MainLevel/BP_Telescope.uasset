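; Coin-operated telescope on the main level that the seagull player uses to enter and leave a telescope camera view.
; An overlap box enables input and highlights the seagull's action tip.
; The action input toggles the view behind blackscreen fades and locks player control, calling the coin or no-coin camera.
; A held coin is consumed and permanently unlocks the coin view through TelescopeStatus on the game instance.
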(event `InputAction|Pickup/Drop/Throw`
  (params (Key :type "Key Structure"))
  (:`Pressed`
    (`KismetSystemLibrary.Delay` 0.2)))

(event `self.Box.OnComponentBeginOverlap`
  (params (OverlappedComponent :type "PrimitiveComponent Object Reference") (OtherActor :type "Actor Object Reference") (OtherComp :type "PrimitiveComponent Object Reference") (OtherBodyIndex :type Integer) (bFromSweep :type Boolean) (SweepResult :type "HitResult Structure (by ref)"))
  (bind _asbp_seagull (cast `/Game/Blueprints/BP_Seagull` OtherActor))
  (`self.EnableInput` (`GameplayStatics.GetPlayerController` 0))
  (`PrimitiveComponent.SetMaterial` (`/Game/Blueprints/BP_Seagull.actionTip_part` _asbp_seagull) 0 "/Game/Materials/MI_Solid_Yellow.MI_Solid_Yellow")
  (`PrimitiveComponent.SetMaterial` (`/Game/Blueprints/BP_Seagull.actionTip` _asbp_seagull) 0 "/Game/Materials/MI_Solid_Yellow.MI_Solid_Yellow"))

(event `self.Box.OnComponentEndOverlap`
  (params (OverlappedComponent :type "PrimitiveComponent Object Reference") (OtherActor :type "Actor Object Reference") (OtherComp :type "PrimitiveComponent Object Reference") (OtherBodyIndex :type Integer))
  (bind _asbp_seagull (cast `/Game/Blueprints/BP_Seagull` OtherActor))
  (`self.DisableInput` (`GameplayStatics.GetPlayerController` 0))
  (`PrimitiveComponent.SetMaterial` (`/Game/Blueprints/BP_Seagull.actionTip` _asbp_seagull) 0 "/Game/Materials/MI_Transparent_Inst.MI_Transparent_Inst")
  (`PrimitiveComponent.SetMaterial` (`/Game/Blueprints/BP_Seagull.actionTip_part` _asbp_seagull) 0 "/Game/Materials/MI_Transparent_Inst.MI_Transparent_Inst"))

(event `InputAction|Action` :consume false
  (params (Key :type "Key Structure"))
  (:`Pressed`
    (bind _asbp_seagull (cast `/Game/Blueprints/BP_Seagull` (`GameplayStatics.GetPlayerCharacter` 0) :!label _label))
    (if (`self.inCam`)
      (set `/Game/Blueprints/BP_Seagull.canControl` true _asbp_seagull)
      (bind _ui_blackscreen_var (`/Game/Blueprints/BP_Seagull.UI_Blackscreen_var` _asbp_seagull))
      (`/Game/Blueprints/UI/UI_BlackScreen.FastFadeOut` _ui_blackscreen_var)
      (`KismetSystemLibrary.Delay` 0.5)
      (`self.Camera_Reset`)
      (`/Game/Blueprints/UI/UI_BlackScreen.Fade In` _ui_blackscreen_var)
      (set `self.inCam` false)
      (`self.DisableInput` null)
      (`PrimitiveComponent.SetMaterial` (`/Game/Blueprints/BP_Seagull.actionTip_part` _asbp_seagull) 0 "/Game/Materials/MI_Transparent_Inst.MI_Transparent_Inst")
      (`PrimitiveComponent.SetMaterial` (`/Game/Blueprints/BP_Seagull.actionTip` _asbp_seagull) 0 "/Game/Materials/MI_Transparent_Inst.MI_Transparent_Inst")
      (else
        (set `/Game/Blueprints/BP_Seagull.canControl` false _asbp_seagull)
        (bind _asgame_instance_master (cast `/Game/Blueprints/GameInstance_Master` (`GameplayStatics.GetGameInstance`)))
        (if (`/Game/Blueprints/GameInstance_Master.Telescope_Status` _asgame_instance_master)
          (bind _ui_blackscreen_var_2 (`/Game/Blueprints/BP_Seagull.UI_Blackscreen_var` _asbp_seagull))
          (`/Game/Blueprints/UI/UI_BlackScreen.FastFadeOut` _ui_blackscreen_var_2)
          (`KismetSystemLibrary.Delay` 0.5)
          (`self.Camera_Coin`)
          (`/Game/Blueprints/UI/UI_BlackScreen.Fade In` _ui_blackscreen_var_2)
          (set `self.inCam` true)
          (elif (`KismetStringLibrary.EqualEqual_StrStr` (`/Game/Blueprints/BP_Seagull.PickedItemId` _asbp_seagull) "coin")
            (bind _asgame_instance_master_2 (cast `/Game/Blueprints/GameInstance_Master` (`GameplayStatics.GetGameInstance`)))
            (set `/Game/Blueprints/GameInstance_Master.Telescope_Status` true _asgame_instance_master_2)
            (`/Game/Blueprints/UI/UI_BlackScreen.FastFadeOut` _ui_blackscreen_var_2)
            (`KismetSystemLibrary.Delay` 0.5)
            (`self.Camera_Coin`)
            (`/Game/Blueprints/UI/UI_BlackScreen.Fade In` _ui_blackscreen_var_2)
            (set `self.inCam` true)
            (`/Game/Blueprints/BP_Seagull.Clear Item` _asbp_seagull)
            (`KismetSystemLibrary.Delay` 0.2)
            (`self.EnableInput` (`GameplayStatics.GetPlayerController` 0))
            (else
              (bind _ui_blackscreen_var_3 (`/Game/Blueprints/BP_Seagull.UI_Blackscreen_var` _asbp_seagull))
              (`/Game/Blueprints/UI/UI_BlackScreen.FastFadeOut` _ui_blackscreen_var_3)
              (`KismetSystemLibrary.Delay` 0.5)
              (`self.Camera_NoCoin`)
              (`/Game/Blueprints/UI/UI_BlackScreen.Fade In` _ui_blackscreen_var_3)
              (set `self.inCam` true))))))))

(event `InputAction`
  (goto _label))

(fn `UserConstructionScript`)