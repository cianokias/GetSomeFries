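; BP_Trigger_SeagullTalk is a trigger box that lets the player start a seagull talk.
; When a BP_Seagull enters while the game instance allows talking, it enables input and turns the seagull's action tip yellow.
; Exit disables input and makes the tip transparent.
; Pressing Action calls SeagullTalk if talking is allowed and not already running, while Pickup/Drop/Throw only runs an unconnected delay.
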(event `self.Box.OnComponentBeginOverlap`
  (params (OverlappedComponent :type "PrimitiveComponent Object Reference") (OtherActor :type "Actor Object Reference") (OtherComp :type "PrimitiveComponent Object Reference") (OtherBodyIndex :type Integer) (bFromSweep :type Boolean) (SweepResult :type "HitResult Structure (by ref)"))
  (bind _asgame_instance_master (cast `/Game/Blueprints/GameInstance_Master` (`GameplayStatics.GetGameInstance`)))
  (if (`/Game/Blueprints/GameInstance_Master.canSeagullTalk` _asgame_instance_master)
    (bind _asbp_seagull (cast `/Game/Blueprints/BP_Seagull` OtherActor))
    (`self.EnableInput` (`GameplayStatics.GetPlayerController` 0))
    (`PrimitiveComponent.SetMaterial` (`/Game/Blueprints/BP_Seagull.actionTip_part` _asbp_seagull) 0 "/Game/Materials/MI_Solid_Yellow.MI_Solid_Yellow")
    (`PrimitiveComponent.SetMaterial` (`/Game/Blueprints/BP_Seagull.actionTip` _asbp_seagull) 0 "/Game/Materials/MI_Solid_Yellow.MI_Solid_Yellow")))

(event `self.Box.OnComponentEndOverlap`
  (params (OverlappedComponent :type "PrimitiveComponent Object Reference") (OtherActor :type "Actor Object Reference") (OtherComp :type "PrimitiveComponent Object Reference") (OtherBodyIndex :type Integer))
  (bind _asbp_seagull (cast `/Game/Blueprints/BP_Seagull` OtherActor))
  (`self.DisableInput` (`GameplayStatics.GetPlayerController` 0))
  (`PrimitiveComponent.SetMaterial` (`/Game/Blueprints/BP_Seagull.actionTip` _asbp_seagull) 0 "/Game/Materials/MI_Transparent_Inst.MI_Transparent_Inst")
  (`PrimitiveComponent.SetMaterial` (`/Game/Blueprints/BP_Seagull.actionTip_part` _asbp_seagull) 0 "/Game/Materials/MI_Transparent_Inst.MI_Transparent_Inst"))

(event `InputAction|Pickup/Drop/Throw` :consume false
  (params (Key :type "Key Structure"))
  (:`Pressed`
    (`KismetSystemLibrary.Delay` 0.2)))

(event `InputAction|Action`
  (params (Key :type "Key Structure"))
  (:`Pressed`
    (bind _asgame_instance_master (cast `/Game/Blueprints/GameInstance_Master` (`GameplayStatics.GetGameInstance`)))
    (if (`/Game/Blueprints/GameInstance_Master.canSeagullTalk` _asgame_instance_master)
      (if (not (`/Game/Blueprints/GameInstance_Master.inSeagullTalk` _asgame_instance_master))
        (`self.SeagullTalk`)))))

(fn `UserConstructionScript`)