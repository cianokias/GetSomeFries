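; Main-level wall button that the seagull player uses with a held card to trigger a stop-fan-rotation call.
; Box overlap toggles input and the seagull's action-tip highlight.
; A correct press turns the button green, disables interaction and saves the switch in the GameInstance; a wrong press flashes red with a brief lockout.
; BeginPlay restores the used, green state from that saved flag without repeating the fan call.
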(event `InputAction|Pickup/Drop/Throw`
  (params (Key :type "Key Structure"))
  (:`Pressed`
    (`KismetSystemLibrary.Delay` 0.2)))

(event `self.Box.OnComponentBeginOverlap`
  (params (OverlappedComponent :type "PrimitiveComponent Object Reference") (OtherActor :type "Actor Object Reference") (OtherComp :type "PrimitiveComponent Object Reference") (OtherBodyIndex :type Integer) (bFromSweep :type Boolean) (SweepResult :type "HitResult Structure (by ref)"))
  (if (`self.canInteract`)
    (bind _asbp_seagull (cast `/Game/Blueprints/BP_Seagull` OtherActor))
    (`self.EnableInput` (`GameplayStatics.GetPlayerController` 0))
    (`PrimitiveComponent.SetMaterial` (`/Game/Blueprints/BP_Seagull.actionTip_part` _asbp_seagull) 0 "/Game/Materials/MI_Solid_Yellow.MI_Solid_Yellow")
    (`PrimitiveComponent.SetMaterial` (`/Game/Blueprints/BP_Seagull.actionTip` _asbp_seagull) 0 "/Game/Materials/MI_Solid_Yellow.MI_Solid_Yellow")))

(event `self.Box.OnComponentEndOverlap`
  (params (OverlappedComponent :type "PrimitiveComponent Object Reference") (OtherActor :type "Actor Object Reference") (OtherComp :type "PrimitiveComponent Object Reference") (OtherBodyIndex :type Integer))
  (bind _asbp_seagull (cast `/Game/Blueprints/BP_Seagull` OtherActor))
  (`self.DisableInput` (`GameplayStatics.GetPlayerController` 0))
  (`PrimitiveComponent.SetMaterial` (`/Game/Blueprints/BP_Seagull.actionTip` _asbp_seagull) 0 "/Game/Materials/MI_Transparent_Inst.MI_Transparent_Inst")
  (`PrimitiveComponent.SetMaterial` (`/Game/Blueprints/BP_Seagull.actionTip_part` _asbp_seagull) 0 "/Game/Materials/MI_Transparent_Inst.MI_Transparent_Inst"))

(event `InputAction|Action`
  (params (Key :type "Key Structure"))
  (:`Pressed`
    (bind _asbp_seagull (cast `/Game/Blueprints/BP_Seagull` (`GameplayStatics.GetPlayerCharacter` 0)))
    (if (`KismetStringLibrary.EqualEqual_StrStr` (`/Game/Blueprints/BP_Seagull.PickedItemId` _asbp_seagull) "card")
      (`/Engine/EditorBlueprintResources/StandardMacros.DoOnce` false
        (:`Completed`
          (set `self.canInteract` false)
          (`self.StopFanRotate`)
          (`PrimitiveComponent.SetMaterial` (`self.button`) 4 "/Game/Materials/MI_Solid_LightGreen.MI_Solid_LightGreen" :!label _label)
          (bind _asgame_instance_master (cast `/Game/Blueprints/GameInstance_Master` (`GameplayStatics.GetGameInstance`)))
          (set `/Game/Blueprints/GameInstance_Master.MainLevel_Switch_Fan` true _asgame_instance_master)))
      (else
        (`PrimitiveComponent.SetMaterial` (`self.button`) 4 "/Game/3DModels/storage_/button_red.button_red")
        (set `self.canInteract` false)
        (`KismetSystemLibrary.Delay` 2.0)
        (`PrimitiveComponent.SetMaterial` (`self.button`) 4 "/Game/3DModels/storage_/button_bule.button_bule")
        (set `self.canInteract` true)))))

(event `self.ReceiveBeginPlay`
  (bind _asgame_instance_master (cast `/Game/Blueprints/GameInstance_Master` (`GameplayStatics.GetGameInstance`)))
  (if (`/Game/Blueprints/GameInstance_Master.MainLevel_Switch_Fan` _asgame_instance_master)
    (set `self.canInteract` false)
    (goto _label)))

(fn `UserConstructionScript`)