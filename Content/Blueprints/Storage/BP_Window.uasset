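; BP_Window is a storage-area window that acts as a level exit to the kitchen for the player's seagull.
; While CanOpen is set, overlapping its box enables input and lights the seagull's action tip yellow; leaving reverses both.
; The Action input locks seagull control, fades to black, sets the kitchen spawn point on the game instance, calls CallRecordBoxTransform, then opens Kitchen_new after a delay.
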(event `self.Box.OnComponentBeginOverlap`
  (params (OverlappedComponent :type "PrimitiveComponent Object Reference") (OtherActor :type "Actor Object Reference") (OtherComp :type "PrimitiveComponent Object Reference") (OtherBodyIndex :type Integer) (bFromSweep :type Boolean) (SweepResult :type "HitResult Structure (by ref)"))
  (if (`self.canOpen`)
    (bind _asbp_seagull (cast `/Game/Blueprints/BP_Seagull` OtherActor))
    (`self.EnableInput` (`GameplayStatics.GetPlayerController` 0))
    (`PrimitiveComponent.SetMaterial` (`/Game/Blueprints/BP_Seagull.actionTip_part` _asbp_seagull) 0 "/Game/Materials/MI_Solid_Yellow.MI_Solid_Yellow")
    (`PrimitiveComponent.SetMaterial` (`/Game/Blueprints/BP_Seagull.actionTip` _asbp_seagull) 0 "/Game/Materials/MI_Solid_Yellow.MI_Solid_Yellow")))

(event `self.Box.OnComponentEndOverlap`
  (params (OverlappedComponent :type "PrimitiveComponent Object Reference") (OtherActor :type "Actor Object Reference") (OtherComp :type "PrimitiveComponent Object Reference") (OtherBodyIndex :type Integer))
  (bind _asbp_seagull (cast `/Game/Blueprints/BP_Seagull` OtherActor))
  (`self.DisableInput` (`GameplayStatics.GetPlayerController` 0))
  (`PrimitiveComponent.SetMaterial` (`/Game/Blueprints/BP_Seagull.actionTip` _asbp_seagull) 0 "/Game/Materials/MI_Transparent_Inst.MI_Transparent_Inst")
  (`PrimitiveComponent.SetMaterial` (`/Game/Blueprints/BP_Seagull.actionTip_part` _asbp_seagull) 0 "/Game/Materials/MI_Transparent_Inst.MI_Transparent_Inst"))

(event `InputAction|Action`
  (params (Key :type "Key Structure"))
  (:`Pressed`
    (bind _asbp_seagull (cast `/Game/Blueprints/BP_Seagull` (`GameplayStatics.GetPlayerCharacter` 0)))
    (set `/Game/Blueprints/BP_Seagull.canControl` false _asbp_seagull)
    (`/Game/Blueprints/UI/UI_BlackScreen.Fade Out` (`/Game/Blueprints/BP_Seagull.UI_Blackscreen_var` _asbp_seagull))
    (bind _asgame_instance_master (cast `/Game/Blueprints/GameInstance_Master` (`GameplayStatics.GetGameInstance`)))
    (set `/Game/Blueprints/GameInstance_Master.Kitchen_SpawnPoint` 1 _asgame_instance_master)
    (`self.RecordBoxTransform`)
    (`KismetSystemLibrary.Delay` 1.0)
    (`GameplayStatics.OpenLevelBySoftObjectPtr` "/Game/Maps/Kitchen_new.Kitchen_new")))

(event `InputAction|Pickup/Drop/Throw`
  (params (Key :type "Key Structure"))
  (:`Pressed`
    (`KismetSystemLibrary.Delay` 0.2)))

(fn `UserConstructionScript`)