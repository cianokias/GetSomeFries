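; BP_VFXplayer is a test-level trigger actor that plays visual effects when a seagull passes through it.
; When a BP_Seagull begins overlapping its Plane component, it spawns the NS_forVFXplayer system at four marker points.
; Other overlapping actors are ignored, and the effect fires again on each new seagull overlap.
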(event `self.Plane.OnComponentBeginOverlap`
  (params (OverlappedComponent :type "PrimitiveComponent Object Reference") (OtherActor :type "Actor Object Reference") (OtherComp :type "PrimitiveComponent Object Reference") (OtherBodyIndex :type Integer) (bFromSweep :type Boolean) (SweepResult :type "HitResult Structure (by ref)"))
  (cast `/Game/Blueprints/BP_Seagull` OtherActor)
  (`NiagaraFunctionLibrary.SpawnSystemAtLocation` "/Game/Blueprints/testLevel/NS_forVFXplayer.NS_forVFXplayer" (`SceneComponent.K2_GetComponentLocation` (`self.Point1`)))
  (`NiagaraFunctionLibrary.SpawnSystemAtLocation` "/Game/Blueprints/testLevel/NS_forVFXplayer.NS_forVFXplayer" (`SceneComponent.K2_GetComponentLocation` (`self.Point2`)))
  (`NiagaraFunctionLibrary.SpawnSystemAtLocation` "/Game/Blueprints/testLevel/NS_forVFXplayer.NS_forVFXplayer" (`SceneComponent.K2_GetComponentLocation` (`self.Point3`)))
  (`NiagaraFunctionLibrary.SpawnSystemAtLocation` "/Game/Blueprints/testLevel/NS_forVFXplayer.NS_forVFXplayer" (`SceneComponent.K2_GetComponentLocation` (`self.Point4`))))

(fn `UserConstructionScript`)