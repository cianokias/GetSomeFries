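; Level switch trigger actor that moves the game to a referenced test level when the seagull carrying the test key touches it.
; An overlap on its Plane component checks the overlapping BP_Seagull's picked item ID for the key.
; On a match it disables the player seagull's control, calls FadeOut on its blackscreen UI, then opens the level after a short delay.
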(event `self.Plane.OnComponentBeginOverlap`
  (params (OverlappedComponent :type "PrimitiveComponent Object Reference") (OtherActor :type "Actor Object Reference") (OtherComp :type "PrimitiveComponent Object Reference") (OtherBodyIndex :type Integer) (bFromSweep :type Boolean) (SweepResult :type "HitResult Structure (by ref)"))
  (bind _asbp_seagull (cast `/Game/Blueprints/BP_Seagull` OtherActor))
  (if (`KismetStringLibrary.EqualEqual_StrStr` (`/Game/Blueprints/BP_Seagull.PickedItemId` _asbp_seagull) "test_key")
    (bind _asbp_seagull_2 (cast `/Game/Blueprints/BP_Seagull` (`GameplayStatics.GetPlayerCharacter` 0)))
    (set `/Game/Blueprints/BP_Seagull.canControl` false _asbp_seagull_2)
    (`/Game/Blueprints/UI_BlackScreen.Fade Out` (`/Game/Blueprints/BP_Seagull.UI_Blackscreen_var` _asbp_seagull_2))
    (`KismetSystemLibrary.Delay` 1.0)
    (`GameplayStatics.OpenLevelBySoftObjectPtr` "/Game/Maps/testLevel.testLevel")))

(fn `UserConstructionScript`)